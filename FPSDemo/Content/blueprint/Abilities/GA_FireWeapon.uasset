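; GA_FireWeapon is a Gameplay Ability that fires a hitscan shot from the third-person character.
; On activation it casts the avatar to BP_ThirdPersonCharacter and line traces on the Visibility channel along the follow camera's forward vector.
; It draws the trace for debugging, prints the hit actor's name and ends the ability, with no damage or effects applied.
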(event Ability|EventOnEndAbility
  (params (bWasCancelled :type Boolean)))

(event Ability|EventActivateAbility
  (bind _asbp_third_person_character (Utilities|Casting|CastToBP_ThirdPersonCharacter (Ability|GetAvatarActorfromActorInfo)))
  (Variables|Default|Setbp_PlayerRef _asbp_third_person_character)
  (bind _outhit (Collision|LineTraceByChannel (Transformation|GetWorldLocation (Variables|/Game/ThirdPerson/Blueprints/BP_ThirdPersonCharacter.BP_ThirdPersonCharacter_C|GetFollowCamera (Variables|Default|Getbp_PlayerRef))) (+ (Transformation|GetWorldLocation (Variables|/Game/ThirdPerson/Blueprints/BP_ThirdPersonCharacter.BP_ThirdPersonCharacter_C|GetFollowCamera (Variables|Default|Getbp_PlayerRef))) (* (Math|Vector|GetForwardVector (Variables|/Game/ThirdPerson/Blueprints/BP_ThirdPersonCharacter.BP_ThirdPersonCharacter_C|GetFollowCamera (Variables|Default|Getbp_PlayerRef))) 1e+04)) "TraceTypeQuery1" false 0 "ForDuration"))
  (Development|PrintString (Utilities|GetDisplayName (.HitActor (Collision|BreakHitResult _outhit))))
  (Ability|EndAbility))